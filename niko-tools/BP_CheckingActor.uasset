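; BP_CheckingActor is a bootstrap actor that ensures a BP_PlayerInputDetection actor exists during play.
; BeginPlay waits for the loading screen to close outside editor mode, using a looping timer that polls TresUIIsClosedLoadingScreen, and includes a short delay.
; Check and Spawn creates the detection actor only if none exists and optionally attaches it to the player pawn.
; The newly spawned actor receives a reference back to this checker.
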(event `self.ReceiveBeginPlay`
  (if (`self.Editor Mode?`)
    (`KismetSystemLibrary.Delay` 0.2 :!label _label)
    (`|ExecutionSequence`
      (:`then_0`
        (bind _spawned_actor (`self.Check and Spawn` "/Game/niko-tools/BP_PlayerInputDetection.BP_PlayerInputDetection_C" true)
          (:`then`
            (bind _asbp_player_input_detection (cast `/Game/niko-tools/BP_PlayerInputDetection` _spawned_actor))
            (set `/Game/niko-tools/BP_PlayerInputDetection.Checking Actor Reference` self _asbp_player_input_detection)))))
    (else
      (bind _returnvalue (`KismetSystemLibrary.K2_SetTimerDelegate` (delegate `CustomEvent_0`) 0.01 true))
      (set `self.timer` _returnvalue))))

(event `CustomEvent_0`
  (bind _returnvalue (`TresGameBlueprintLibrary.TresUI_IsClosedLoadingScreen`))
  (if _returnvalue
    (`|ExecutionSequence`
      (:`then_0`
        (`KismetSystemLibrary.K2_ClearAndInvalidateTimerHandle` (`self.timer`)))
      (:`then_1`
        (goto _label)))))

(fn `UserConstructionScript`)