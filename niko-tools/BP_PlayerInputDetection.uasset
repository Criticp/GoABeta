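; BP_PlayerInputDetection finds interactables near the player and triggers them on F or the gamepad top face button.
; After a startup delay, a looping timer sphere-traces around the pawn for BP_InteractionCollision actors.
; The closest one, unless already interacting, shows its triangle prompt and becomes the input target; empty traces clear prompts and target.
; Helpers provide a timed Do Once and cursor/look-input toggling; Restrict Attack is empty.
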(event `CustomEvent_0`
  (bind _returnvalue (`GameplayStatics.GetPlayerPawn` 0))
  (bind _returnvalue_2 (`self.K2_GetActorLocation` _returnvalue))
  ;[1 1 1] Event Begin Play
  (bind (_outhits _returnvalue_3) (`KismetSystemLibrary.SphereTraceMulti` _returnvalue_2 _returnvalue_2 370.0 "TraceTypeQuery3" false (`|MakeArray` _returnvalue :!type "Actor Object Reference") (`self.Interaction Trace Debug Mode`) true (struct :`R` 0.802083 :`G` 0.802083 :`B` 0.802083 :`A` 1.0) (struct :`R` 0.266062 :`G` 1.0 :`A` 1.0)))
  (if _returnvalue_3
    (for _array_element _outhits
      (bind _asbp_interaction_collision (cast `/Game/niko-tools/Systems/TriangleInteractionSystem/Actors/BP_InteractionCollision` (`.HitActor` (`GameplayStatics.BreakHitResult` _array_element))))
      (`/Game/niko-tools/Systems/TriangleInteractionSystem/Actors/BP_InteractionCollision.Failsafe` _asbp_interaction_collision self)
      (`KismetArrayLibrary.Array_AddUnique` (`self.Actor Array`) _asbp_interaction_collision)
      (bind (_actor _index _distancesquared _furthestactors1) (`/Game/niko-tools/BlueprintFunctionLibraries/MoreporkFunctions/MoreporkFunctions.GetFurthestOrClosestActor` (`self.K2_GetActorLocation` (`GameplayStatics.GetPlayerPawn` 0)) (`self.Actor Array`) true))
      (set `self.furthest actors` _furthestactors1)
      (bind _asbp_interaction_collision_2 (cast `/Game/niko-tools/Systems/TriangleInteractionSystem/Actors/BP_InteractionCollision` _actor)
        (:`then`
          (bind _interaction_component (`/Game/niko-tools/Systems/TriangleInteractionSystem/Actors/BP_InteractionCollision.Interaction Component` _asbp_interaction_collision_2))
          (if (not (`/Game/niko-tools/Systems/TriangleInteractionSystem/BP_TriangleInteraction.Interacting` _interaction_component))
            (`/Game/niko-tools/Systems/TriangleInteractionSystem/BP_TriangleInteraction.Selected` _interaction_component)
            (`/Game/niko-tools/Systems/TriangleInteractionSystem/BP_TriangleInteraction.Show Triangle Interaction` _interaction_component)
            (set `self.Current Interaction Component` _interaction_component)))
        (:`CastFailed`
          (set `self.Current Interaction Component` null))))
    (else
      (for _array_element_2 (`self.Actor Array`)
        (bind _asbp_interaction_collision_3 (cast `/Game/niko-tools/Systems/TriangleInteractionSystem/Actors/BP_InteractionCollision` _array_element_2)
          (:`then`
            (bind _interaction_component_2 (`/Game/niko-tools/Systems/TriangleInteractionSystem/Actors/BP_InteractionCollision.Interaction Component` _asbp_interaction_collision_3))
            (`/Game/niko-tools/Systems/TriangleInteractionSystem/BP_TriangleInteraction.Hide Triangle Interaction` _interaction_component_2)
            (`/Game/niko-tools/Systems/TriangleInteractionSystem/BP_TriangleInteraction.Unselected` _interaction_component_2)
            (`KismetArrayLibrary.Array_Clear` (`self.Actor Array`)))
          (:`CastFailed`
            _))
        (set `self.Current Collision Actor` null)
        (set `self.Current Interaction Component` null)))))

(event `self.ReceiveBeginPlay`
  ;[1 1 1] Event Begin Play
  (`KismetSystemLibrary.Delay` 2.0)
  (`KismetSystemLibrary.Delay` 0.4)
  (`self.EnableInput` (`GameplayStatics.GetPlayerController` 0))
  (`KismetSystemLibrary.K2_SetTimerDelegate` (delegate `CustomEvent_0`) 0.1 true))

(event `Key|Gamepad_FaceButton_Top`
  (params (Key :type "Key Structure"))
  ;[1 1 1] interact with triangle
  (:`Pressed`
    (bind _current_interaction_component (`self.Current Interaction Component` :!label _label)
      (:`then`
        (`/Game/niko-tools/Systems/TriangleInteractionSystem/BP_TriangleInteraction.Try Interaction` _current_interaction_component))
      (:`else`))))

(event `Key|F`
  (params (Key :type "Key Structure"))
  ;[1 1 1] interact with triangle
  (:`Pressed`
    (goto _label)))

(fn `UserConstructionScript`)