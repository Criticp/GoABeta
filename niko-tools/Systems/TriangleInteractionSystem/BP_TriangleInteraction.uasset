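; Scene component that gives its owning actor a triangle-button interaction prompt with a TresUI action command.
; On BeginPlay it spawns and attaches an interaction collision actor and binds its Selected and Interact events.
; Showing spawns an attached 3D widget actor, while a retriggerable delay hides it once Selected events stop arriving.
; InteractionMode decides whether interacting resets the prompt, hides it temporarily, works once or is disabled.
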(event `self.ReceiveBeginPlay`
  (add `self.Interact` (delegate `CustomEvent_0`))
  (bind _returnvalue (`|SpawnActorFromClass` "/Game/niko-tools/Systems/TriangleInteractionSystem/Actors/BP_InteractionCollision.BP_InteractionCollision_C" (`KismetMathLibrary.MakeTransform` (`self.K2_GetComponentLocation`)) "AlwaysSpawn" "OverrideRootScale" null self null))
  (`Actor.K2_AttachToComponent` _returnvalue self "None" "SnapToTarget" "KeepRelative" "KeepRelative" true)
  (add `self.Selected` (delegate `CustomEvent_1`)))

(event `CustomEvent_1`
  (`|ExecutionSequence`
    (:`then_0`
      (`KismetSystemLibrary.RetriggerableDelay` 0.15)
      (`TresGameBlueprintLibrary.TresUI_DeleteActionCommandMode` (`self.InteractionName`) "ETresUIHudCommandExKind_None")
      (`self.Hide Triangle Interaction`))
    (:`then_1`
      (switch `/Game/niko-tools/Systems/TriangleInteractionSystem/Data/E_InteractionMode` (`self.Interaction Mode`)
        (:`NewEnumerator7`
          (`/Engine/EditorBlueprintResources/StandardMacros.DoOnce` false :!label _label
            (:`Completed`
              (set `self.Selected?` true))))
        (:`NewEnumerator8`
          (goto _label))
        (:`NewEnumerator9`
          (goto _label))
        (:`NewEnumerator10`
          (`self.Hide Triangle Interaction`))))))

(event `Show Triangle Interaction`
  ;[1 1 1] Add the Triangle Interaction Widget to the owning actor of this component
  (switch `/Game/niko-tools/Systems/TriangleInteractionSystem/Data/E_InteractionMode` (`self.Interaction Mode`)
    (:`NewEnumerator7`
      (if (`self.Selected?`) :!label _label_2
        (`/Engine/EditorBlueprintResources/StandardMacros.DoOnce` false :!label _label_3
          (:`Completed`
            (bind _returnvalue (`|SpawnActorFromClass` "/Game/niko-tools/Systems/TriangleInteractionSystem/Actors/BP_Triangle3DWidgetActor.BP_Triangle3DWidgetActor_C" (`KismetMathLibrary.MakeTransform` (`self.K2_GetComponentLocation` (`Actor.GetComponentByClass` (`self.GetOwner`) "BP_TriangleInteraction_C"))) "AlwaysSpawn" "OverrideRootScale" null (struct :`R` 0.269522 :`G` 1.0 :`A` 1.0) null))
            (set `self.triangle actor` _returnvalue)
            (bind _output_get (set `self.Triangle Interaction Widget` (cast `/Game/niko-tools/Systems/TriangleInteractionSystem/UI/W_TriangleHolder` (`WidgetComponent.GetUserWidgetObject` (`/Game/niko-tools/Systems/TriangleInteractionSystem/Actors/BP_Triangle3DWidgetActor.Widget` _returnvalue)) :!pure true)))
            (`/Game/niko-tools/Systems/TriangleInteractionSystem/UI/W_TriangleHolder.Start Triangle Interaction` _output_get (`self.Triangle Color`))
            (`Actor.K2_AttachToComponent` (`self.triangle actor`) self "None" "SnapToTarget" "KeepRelative" "KeepRelative" true)
            (`TresGameBlueprintLibrary.TresUI_AddActionCommandMode` (`self.InteractionName`) "ETresUIHudCommandExKind_None")))))
    (:`NewEnumerator8`
      (goto _label_2))
    (:`NewEnumerator9`
      (`/Engine/EditorBlueprintResources/StandardMacros.DoOnce` false
        (:`Completed`
          (goto _label_2))))
    (:`NewEnumerator10`
      (`self.Hide Triangle Interaction`))))

(event `reset`
  (goto _label :!via `Reset`))

(event `Try Interaction`
  ;[0.05782 0.1813 0.3802 0.384] Try to call the interaction event
  (if (`self.Selected?`)
    (switch `/Game/niko-tools/Systems/TriangleInteractionSystem/Data/E_InteractionMode` (`self.Interaction Mode`)
      (:`NewEnumerator7`
        (`self.Interact` "NewEnumerator0" :!label _label_4))
      (:`NewEnumerator8`
        (goto _label_4))
      (:`NewEnumerator9`
        (goto _label_4))
      (:`NewEnumerator10`
        (`self.Hide Triangle Interaction`)))))

(event `CustomEvent_0` :!signature `self.Interact`
  (params (Interaction :type "/Game/niko-tools/Systems/TriangleInteractionSystem/Data/E_InteractionList Enum" :default "NewEnumerator0"))
  (switch `/Game/niko-tools/Systems/TriangleInteractionSystem/Data/E_InteractionMode` (`self.Interaction Mode`)
    (:`NewEnumerator7`
      ;[0.07174 0.4635 0 0.384] Interact
      (`self.Play Sound`)
      (`self.Reset Triangle Interaction`))
    (:`NewEnumerator8`
      ;[1 0.4348 0 0.384] Hide After Interact
      (set `self.Selected?` false)
      (`self.Hide Triangle Interaction`)
      (`TresGameBlueprintLibrary.TresUI_DeleteActionCommandMode` (`self.InteractionName`) "ETresUIHudCommandExKind_None")
      (set `self.Interacting` true))
    (:`NewEnumerator9`
      ;[0.2344 0 0] Only interact ONCE
      (`KismetArrayLibrary.Array_Clear` (`self.InteractionList`))
      (`self.Hide Triangle Interaction`)
      (`TresGameBlueprintLibrary.TresUI_DeleteActionCommandMode` (`self.InteractionName`) "ETresUIHudCommandExKind_None"))))

(event `Hide Triangle Interaction`
  ;[1 1 1] Add the Triangle Interaction Widget to the owning actor of this component
  (`TresGameBlueprintLibrary.TresUI_DeleteActionCommandMode` (`self.InteractionName`) "ETresUIHudCommandExKind_None")
  (`/Game/niko-tools/Systems/TriangleInteractionSystem/UI/W_TriangleHolder.Stop Triangle Interaction` (`self.Triangle Interaction Widget`))
  (`Actor.K2_DestroyActor` (`self.triangle actor`))
  (goto _label_3 :!via `Reset`))

(event `Play Sound`)

(event `Unselected`
  (set `self.Selected?` false)
  (set `self.Interacting` false)
  (`self.reset`))

(fn `Reset Triangle Interaction`
  (`self.Hide Triangle Interaction`)
  (`self.Unselected`)
  (`self.reset`)
  (set `self.Interacting` false))